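; Bouncing sound ball that plays an FMOD event on spawn and on impacts, shaped by the blocks in its path.
; On each hit it traces along its velocity and maps the surface type to instrument, pitch, volume, flanger, scale or bounce-limit changes.
; After a short delay it plays the sound at the hit location with those parameters.
; It ignores player collision, and hides then destroys itself at its bounce limit or when far from the player.
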(event Collision|EventHit
  (params (MyComp :type Primitive%20Component%20Object%20Reference) (Other :type Actor%20Object%20Reference) (OtherComp :type Primitive%20Component%20Object%20Reference) (bSelfMoved :type Boolean) (HitLocation :type Vector :default "0, 0, 0") (HitNormal :type Vector :default "0, 0, 0") (NormalImpulse :type Vector :default "0, 0, 0") (Hit :type Hit%20Result%20Structure%20%28by%20ref%29))
  ;[0.15 0 0 0.5] New Line Trace after Bounce // Destroy on 4th Bounce // Play Sound on Bounce
  (Utilities|FlowControl|Sequence
    (:then_0
      (Transformation|SetActorRotation (* (Math|Conversions|RotationFromXVector (Transformation|GetVelocity)) -1.0))
      (CallFunction|LineTraceSoundBlock))
    (:then_1
      (Utilities|FlowControl|RetriggerableDelay 0.01)
      (bind _result (Math|Integer|IncrementInt (Variables|Default|GetBounces))
        (:%20%20
          (if (>= _result (Variables|Default|GetMaxBounces))
            (CallFunction|HideBall)
            (Variables|Default|SetisHidden? true)
            (Utilities|FlowControl|Delay 1.0)
            (Actor|DestroyActor)
            (else
              (bind _returnvalue (Class|FMODBlueprintStatics|PlayEventatLocation "/Game/FMOD/Events/SFX_Sounds/SFX_SoundBall.SFX_SoundBall" (Math|Conversions|ToTransform(Vector) HitLocation)))
              (Class|FMODBlueprintStatics|EventInstanceSetParameter _returnvalue "Instrument" (Variables|Default|GetInstrument))
              (Class|FMODBlueprintStatics|EventInstanceSetParameter _returnvalue "Pitch" (Variables|Default|GetPitch))
              (Class|FMODBlueprintStatics|EventInstanceSetParameter _returnvalue "Flanger" (Variables|Default|GetFlanger))
              (Class|FMODBlueprintStatics|EventInstanceSetParameter _returnvalue "Volume" (Variables|Default|GetVolume))
              (Class|FMODBlueprintStatics|EventInstancePlay _returnvalue))))))))

(event EventBeginPlay
  ;[0.15 0 0 0.5] Line Trace
  (Transformation|SetActorScale3D (Variables|Default|GetScale))
  (bind _returnvalue (Class|FMODBlueprintStatics|PlayEventatLocation "/Game/FMOD/Events/SFX_Sounds/SFX_SoundBall.SFX_SoundBall" (Transformation|GetWorldTransform (Variables|Default|GetSphere))))
  (Class|FMODBlueprintStatics|EventInstanceSetParameter _returnvalue "Volume" (Variables|Default|GetVolume))
  (Class|FMODBlueprintStatics|EventInstancePlay _returnvalue)
  (Variables|Default|SetisActive? true))

(event EventTick
  (params (DeltaSeconds :type Float%20%28single-precision%29))
  ;[0.15 0 0 0.5] Ignore Player Collision
  (bind _asbp_sound_character (Utilities|Casting|CastToBP_SoundCharacter (Game|Player|GetPlayerPawn 0)))
  (Collision|IgnoreActorwhenMoving (Variables|Default|GetSphere) _asbp_sound_character true)
  (if (>= (Transformation|GetDistanceTo _asbp_sound_character (Components|GetOwner (Variables|Default|GetSphere))) 2e+03)
    (Utilities|FlowControl|DoOnce false
      (:Completed
        (CallFunction|HideBall)
        (Utilities|FlowControl|Delay 1.0)
        (Actor|DestroyActor)))))

(fn ConstructionScript)

(fn LineTraceSoundBlock
  (bind _sphere (Variables|Default|GetSphere))
  (bind _returnvalue (Transformation|GetWorldLocation _sphere))
  (Class|FMODAudioComponent|SetParameter (Variables|Default|GetSBall) "Volume" (Variables|Default|GetVolume))
  (bind _outhit (Collision|LineTraceByChannel _returnvalue (+ _returnvalue (Transformation|GetVelocity)) "TraceTypeQuery1" false 0 "None"))
  (switch Utilities|FlowControl|Switch|SwitchonEPhysicalSurface (Collision|GetSurfaceType _outhit)
    (:SurfaceType_Default
      (Variables|Default|SetBlockType 0.0)
      (Class|FMODAudioComponent|SetParameter (Variables|Default|GetSBall) "Instrument" (Variables|Default|GetBlockType) :!label _label)
      (Variables|Default|SetInstrument (Variables|Default|GetBlockType)))
    (:SurfaceType1
      (Variables|Default|SetBlockType 1.0)
      (goto _label))
    (:SurfaceType2
      (Variables|Default|SetBlockType 2.0)
      (goto _label))
    (:SurfaceType3
      (Variables|Default|SetBlockType 3.0)
      (goto _label))
    (:SurfaceType4
      (Variables|Default|SetBlockType 4.0)
      (goto _label))
    (:SurfaceType5
      (Variables|Default|SetBlockType 5.0)
      (goto _label))
    (:SurfaceType6
      (Variables|Default|SetBlockType 6.0)
      (Variables|Default|SetPitch (+ (Variables|Default|GetPitch) 0.25))
      (Class|FMODAudioComponent|SetParameter (Variables|Default|GetSBall) "Pitch" (Variables|Default|GetPitch) :!label _label_2))
    (:SurfaceType7
      (Variables|Default|SetBlockType 7.0)
      (Variables|Default|SetPitch (- (Variables|Default|GetPitch) 0.25))
      (goto _label_2))
    (:SurfaceType8
      (Variables|Default|SetBlockType 8.0)
      (Variables|Default|SetVolume (+ (Variables|Default|GetVolume) 0.1))
      (Class|FMODAudioComponent|SetParameter (Variables|Default|GetSBall) "Volume" (Variables|Default|GetVolume) :!label _label_3))
    (:SurfaceType9
      (Variables|Default|SetBlockType 9.0)
      (Variables|Default|SetVolume (- (Variables|Default|GetVolume) 0.1))
      (goto _label_3))
    (:SurfaceType10
      (Variables|Default|SetBlockType 1e+01)
      (Variables|Default|SetFlanger 1.0)
      (Class|FMODAudioComponent|SetParameter (Variables|Default|GetSBall) "Flanger" (Variables|Default|GetFlanger)))
    (:SurfaceType11
      (Variables|Default|SetBlockType 11.0))
    (:SurfaceType12
      (Variables|Default|SetBlockType 12.0)
      (Variables|Default|SetScale (+ (Variables|Default|GetScale) "0.100000,0.100000,0.100000"))
      (Transformation|SetActorScale3D (Variables|Default|GetScale) :!label _label_4))
    (:SurfaceType13
      (Variables|Default|SetBlockType 13.0)
      (Variables|Default|SetScale (- (Variables|Default|GetScale) "-0.100000,-0.100000,-0.100000"))
      (goto _label_4))
    (:SurfaceType14
      (Variables|Default|SetBlockType 14.0)
      (Variables|Default|SetMaxBounces 5))))

(fn OnRepFMODEvent)

(fn HideBall
  (Rendering|SetActorHiddenInGame true)
  (Collision|SetCollisionEnabled (Variables|Default|GetSphere) "NoCollision")
  (bind _finalvalue (Class|FMODAudioComponent|GetParameterValue (Variables|Default|GetSBall) "Instrument"))
  (Variables|Default|SetInstrument _finalvalue))